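; BP_KeyItem is a key item pickup that a player takes into their inventory.
; Interact forwards to a server pickup event, which plays the pickup sound at the item, adds its ItemType to the BP_FirstPersonCharacter inventory, then destroys the actor.
; GetInteractText builds a "take" prompt from the item's name.
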(event `Server_PickUpItem`
  (params (PlayerActor :type "Actor Object Reference"))
  (`GameplayStatics.PlaySoundAtLocation` (`self.PickUpSound`) (`self.K2_GetActorLocation`) (struct) 1.0 1.0 0.0 null null null null)
  (bind _asbp_first_person_character (cast `/Game/FirstPerson/Blueprints/BP_FirstPersonCharacter` PlayerActor))
  (`KismetArrayLibrary.Array_Add` (`/Game/FirstPerson/Blueprints/BP_FirstPersonCharacter.Inventory` _asbp_first_person_character) (`self.ItemType`))
  (`self.K2_DestroyActor`))

(event `/Game/FirstPerson/Blueprints/BPI_Interact.Interact`
  (params (PlayerActor :type "Actor Object Reference") (InteractedButton :type "Actor Object Reference"))
  (`self.Server_PickUpItem` PlayerActor))

(fn `GetInteractText`
  (returns (Text :type Text))
  (return (`|FormatText` "take {Name}" (`self.ItemName`))))

(fn `UserConstructionScript`)