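; Lever2 is an interactable puzzle lever Blueprint with an on/off state and a matching "on [E]" or "off [E]" prompt.
; OnRep_isActivited plays or reverses the lever timeline to follow that state, and the timeline's update rotates LeverPivot between two angles.
; The EventGraph's toggle logic, which also calls ServerOnInteract on ParentPuzzle, is unreachable, so nothing in this file changes the state.
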(fn `GetInteractText`
  (returns (Text :type Text))
  (if (`self.isActivited`)
    (return "off [E]")
    (else
      (return "on [E]"))))

(fn `OnRep_isActivited`
  (bind _tl_lever (`self.TL_Lever`))
  (if (`self.isActivited`)
    (`TimelineComponent.Play` _tl_lever)
    (else
      (`TimelineComponent.Reverse` _tl_lever))))

(fn `UserConstructionScript`)