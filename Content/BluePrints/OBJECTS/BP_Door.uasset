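; Networked interactable door that swings its pivot 90 degrees and shows an "Open [E]" prompt.
; A timeline lerps between the starting and open rotations, playing a slam or opening sound when finished.
; Interact flips IsOpen and animates via multicast; external triggers set IsOpen, whose OnRep also drives the timeline, with opposite polarity to the toggle.
; ForceCloseDoor reverses the timeline without changing IsOpen, and Server_Interact is empty.
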(event `self.ReceiveBeginPlay`
  (bind _output_get (set `self.ClosedRotation` (`SceneComponent.RelativeRotation` (`self.DoorPivot`))))
  (set `self.OpenRotation` (`KismetMathLibrary.ComposeRotators` _output_get (struct :`Yaw` 90.0))))

(event `Server_Interact`)

(event `Multicast_toggleDoor`
  (bind _returnvalue (`self.K2_GetActorLocation`))
  (if (`self.IsOpen`)
    (set `self.IsOpen` false)
    (bind (_direction _alpha) (`Timeline|TL_Door` :!via `PlayFromStart` :!label _label)
      (:`Update`
        (`SceneComponent.K2_SetRelativeRotation` (`self.DoorPivot`) (`KismetMathLibrary.RLerp` (`self.ClosedRotation`) (`self.OpenRotation`) _alpha true) false false))
      (:`Finished`
        (if (`self.IsOpen`)
          (`GameplayStatics.PlaySoundAtLocation` "/Game/Sounds/soundreality-metal-door-slam-172172__1_.soundreality-metal-door-slam-172172__1_" _returnvalue (struct) 1.0 1.0 0.0 null null null null)
          (else
            (`GameplayStatics.PlaySoundAtLocation` "/Game/Sounds/universfield-opening-metal-door-199581.universfield-opening-metal-door-199581" _returnvalue (struct) 1.0 1.0 0.0 null null null null)))))
    (else
      (set `self.IsOpen` true)
      (goto _label :!via `ReverseFromEnd`))))

(event `/Game/FirstPerson/Blueprints/BPI_Interact.Interact`
  (params (PlayerActor :type "Actor Object Reference") (InteractedButton :type "Actor Object Reference"))
  (`self.Multicast_toggleDoor`))

(event `ForceCloseDoor`
  (goto _label :!via `ReverseFromEnd`))

(event `/Game/FirstPerson/Blueprints/BPI_PuzzleTriggerrable.TriggerActivation`
  (params (IsActivated :type Boolean))
  (set `self.IsOpen` IsActivated))

(fn `GetInteractText`
  (returns (Text :type Text))
  (return "Open [E]"))

(fn `OnRep_IsOpen`
  (bind _tl_door (`self.TL_Door`))
  (if (`self.IsOpen`)
    (`TimelineComponent.PlayFromStart` _tl_door)
    (else
      (`TimelineComponent.ReverseFromEnd` _tl_door))))

(fn `UserConstructionScript`)