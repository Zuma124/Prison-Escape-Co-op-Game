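; BP_Lever is an interactable puzzle lever that toggles between on and off, with matching interact prompt text.
; Interact notifies its ParentPuzzle, flips IsActivited and plays or reverses a timeline that rotates LeverPivot between two angles.
; The state's OnRep drives the same animation on replication, and TriggerActivation sets the state directly.
; A separate server toggle event is gated by a DoOnce with no reset.
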(event `Server_toggleLever`
  (`/Engine/EditorBlueprintResources/StandardMacros.DoOnce` false
    (:`Completed`
      (set `self.isActivited` (not (`self.isActivited`))))))

(event `/Game/FirstPerson/Blueprints/BPI_Interact.Interact`
  (params (PlayerActor :type "Actor Object Reference") (InteractedButton :type "Actor Object Reference"))
  (`/Game/BluePrints/Puzzls/BP_PuzzleBase.Server_OnInteract` (`self.parentPuzzle`) PlayerActor InteractedButton)
  (if (`self.isActivited`)
    (set `self.isActivited` false)
    (bind (_direction _lever) (`Timeline|TL_Lever` :!via `Reverse` :!label _label)
      (:`Update`
        (`SceneComponent.K2_SetRelativeRotation` (`self.LeverPivot`) (`KismetMathLibrary.RLerp` (struct :`Roll` 30.0) (struct :`Roll` 130.0) _lever) false false)))
    (else
      (set `self.isActivited` true)
      (goto _label))))

(event `/Game/FirstPerson/Blueprints/BPI_PuzzleTriggerrable.TriggerActivation`
  (params (IsActivated :type Boolean))
  (set `self.isActivited` IsActivated))

(fn `GetInteractText`
  (returns (Text :type Text))
  (if (`self.isActivited`)
    (return "off [E]")
    (else
      (return "on [E]"))))

(fn `OnRep_isActivited`
  (bind _tl_lever (`self.TL_Lever`))
  (if (`self.isActivited`)
    (`TimelineComponent.Play` _tl_lever)
    (else
      (`TimelineComponent.Reverse` _tl_lever))))

(fn `UserConstructionScript`)