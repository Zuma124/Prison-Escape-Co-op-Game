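; BP_FlikerLight is a light object that plays a flicker effect on a spotlight with matching sound through a multicast event.
; When IsFlickering is already true, the event starts FlikerSound and a timeline that drives spotlight intensity.
; The same curve value is inversely mapped to sound volume, so the sound quiets as the light brightens.
; IsFlickering clears when the timeline finishes, and nothing here sets it from false to true.
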(event `Multicast_StartFlicker`
  (`KismetSystemLibrary.PrintString` "світло")
  (if (`self.IsFlickering`)
    (set `self.IsFlickering` true)
    (`AudioComponent.Play` (`self.FlikerSound`) 0.0)
    (bind (_direction _f) (`Timeline|FlikerTimeLine` :!via `PlayFromStart`)
      (:`Update`
        (`LightComponent.SetIntensity` (`self.SpotLight`) _f)
        (`AudioComponent.SetVolumeMultiplier` (`self.FlikerSound`) (`KismetMathLibrary.MapRangeClamped` _f 0.0 5000.0 1.0 0.1)))
      (:`Finished`
        (set `self.IsFlickering` false)))))

(fn `UserConstructionScript`)