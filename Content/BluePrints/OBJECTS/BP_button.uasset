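; Interactable puzzle button that shows a "press [E]" prompt and animates when pressed.
; Interact forwards the player and button to the parent puzzle, then replays the press timeline or sets IsPressed, whose RepNotify plays it.
; The timeline slides the mesh along Y, and on finish the authority fires the button-pressed call and clears IsPressed.
; TriggerActivation also sets IsPressed directly.
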(event `Server_PressButton`)

(event `/Game/FirstPerson/Blueprints/BPI_Interact.Interact`
  (params (PlayerActor :type "Actor Object Reference") (InteractedButton :type "Actor Object Reference"))
  (bind _buttonmesh (`self.ButtonMesh`))
  (bind (_relativelocation_x _relativelocation_y _relativelocation_z) (`KismetMathLibrary.BreakVector` (`SceneComponent.RelativeLocation` _buttonmesh)))
  (`/Game/BluePrints/Puzzls/BP_PuzzleBase.Server_OnInteract` (`self.parentPuzzle`) PlayerActor InteractedButton)
  (if (`self.isPressed`)
    (bind (_direction _button) (`Timeline|TL_ButtonPress` :!via `PlayFromStart`)
      (:`Update`
        (`SceneComponent.K2_SetRelativeLocation` _buttonmesh (`KismetMathLibrary.MakeVector` _relativelocation_x _button _relativelocation_z) false false))
      (:`Finished`
        (`/Engine/EditorBlueprintResources/ActorMacros.Switch Has Authority`
          (:`Authority`
            (`self.OnButtonPressed`)
            (set `self.isPressed` false)))))
    (else
      (set `self.isPressed` true))))

(event `/Game/FirstPerson/Blueprints/BPI_PuzzleTriggerrable.TriggerActivation`
  (params (IsActivated :type Boolean))
  (set `self.isPressed` IsActivated))

(fn `GetInteractText`
  (returns (Text :type Text))
  (return "press [E]"))

(fn `OnRep_isPressed`
  (if (`self.isPressed`)
    (`TimelineComponent.PlayFromStart` (`self.TL_ButtonPress`))))

(fn `UserConstructionScript`)