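; Game mode for a prison game with Prisoner and Guide roles that spawns and possesses player pawns.
; BeginPlay gives player 0 a first-person character, and PostLogin gives each joining player a Guide, both at hardcoded locations.
; SpawnPlayerByRole can instead spawn either role at a tagged PlayerStart, but its only caller, the join-order role assignment, is disconnected and never runs.
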(event `SpawnPlayerByRole`
  (params (PlayerController :type "PlayerController Object Reference") (Role :type "/Game/BluePrints/EnumS/E_PlayerRole Enum" :default "NewEnumerator0"))
  (if (`|EnumEquality` Role "NewEnumerator0")
    (bind _outactors (`GameplayStatics.GetAllActorsOfClass` "/Script/Engine.PlayerStart"))
    (for _array_element _outactors
      (if (`self.ActorHasTag` _array_element "PrisonerSpawn")
        (bind _returnvalue (`|SpawnActorFromClass` "/Game/FirstPerson/Blueprints/BP_Prisoner.BP_Prisoner_C" (`self.GetTransform` _array_element) "AdjustIfPossibleButAlwaysSpawn" "MultiplyWithRoot" null null))
        (`Controller.Possess` PlayerController _returnvalue)
        (break)))
    (else
      (bind _outactors_2 (`GameplayStatics.GetAllActorsOfClass` "/Script/Engine.PlayerStart"))
      (for _array_element_2 _outactors_2
        (if (`self.ActorHasTag` _array_element_2 "GuideSpawn")
          (bind _returnvalue_2 (`|SpawnActorFromClass` "/Game/FirstPerson/Blueprints/BP_Guide.BP_Guide_C" (`self.GetTransform` _array_element_2) "AdjustIfPossibleButAlwaysSpawn" "MultiplyWithRoot" null null))
          (`Controller.Possess` PlayerController _returnvalue_2)
          (break))))))

(event `self.ReceiveBeginPlay`
  (bind _returnvalue (`|SpawnActorFromClass` "/Game/FirstPerson/Blueprints/BP_FirstPersonCharacter.BP_FirstPersonCharacter_C" (`KismetMathLibrary.MakeTransform` (50.0 -10.0 180.0)) "AdjustIfPossibleButAlwaysSpawn" "MultiplyWithRoot" null null))
  (`Controller.Possess` (`GameplayStatics.GetPlayerController` 0) _returnvalue))

(event `self.K2_PostLogin`
  (params (NewPlayer :type "PlayerController Object Reference"))
  (bind _returnvalue (`|SpawnActorFromClass` "/Game/FirstPerson/Blueprints/BP_Guide.BP_Guide_C" (`KismetMathLibrary.MakeTransform` (1930.0 3670.0 2400.0)) "AdjustIfPossibleButAlwaysSpawn" "MultiplyWithRoot" null null))
  (`Controller.Possess` NewPlayer _returnvalue))

(fn `UserConstructionScript`)