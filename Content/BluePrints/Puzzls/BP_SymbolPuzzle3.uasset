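; BP_SymbolPuzzle3 is a button-sequence puzzle built from three BP_button child actors, which receive the puzzle as their parent on BeginPlay.
; Each interaction appends the first tag of the pressed button's parent component to CurrentSequence.
; At thirteen entries the sequence is compared with CorrectSequence, calling SolvePuzzle or ServerHandleFailedState.
; ResetPuzzle clears the input; CurrentSequence has an empty OnRep, and debug prints remain.
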(event `self.ReceiveInteraction`
  (params (`Player Actor` :type "Actor Object Reference") (`Interacted Button` :type "Actor Object Reference"))
  (bind _currentsequence (`self.CurrentSequence`))
  (bind _returnvalue (`KismetArrayLibrary.Array_Length` (`self.CurrentSequence`)))
  (`KismetSystemLibrary.PrintString` "1")
  (bind _asbp_button (cast `/Game/BluePrints/OBJECTS/BP_button` `Interacted Button`))
  (bind _returnvalue_2 (`KismetArrayLibrary.Array_Add` _currentsequence (`|GetArrayItem` (`ActorComponent.ComponentTags` (`self.GetParentComponent` _asbp_button)))))
  (`KismetSystemLibrary.PrintString` (`KismetStringLibrary.Conv_IntToString` _returnvalue_2))
  (`KismetSystemLibrary.PrintString` (`KismetStringLibrary.Conv_IntToString` _returnvalue))
  (if (== _returnvalue 13)
    (if (`KismetArrayLibrary.Array_Identical` (`self.CorrectSequence`) _currentsequence)
      (`self.SolvePuzzle`)
      (else
        (`self.Server_HandleFailedState`)))))

(event `self.ReceiveBeginPlay`
  (`parent.ReceiveBeginPlay`)
  (bind _asbp_button (cast `/Game/BluePrints/OBJECTS/BP_button` (`ChildActorComponent.ChildActor` (`self.BP_button`))))
  (set `/Game/BluePrints/OBJECTS/BP_button.parentPuzzle` self _asbp_button)
  (bind _asbp_button_2 (cast `/Game/BluePrints/OBJECTS/BP_button` (`ChildActorComponent.ChildActor` (`self.BP_button1`))))
  (set `/Game/BluePrints/OBJECTS/BP_button.parentPuzzle` self _asbp_button_2)
  (bind _asbp_button_3 (cast `/Game/BluePrints/OBJECTS/BP_button` (`ChildActorComponent.ChildActor` (`self.BP_button2`))))
  (set `/Game/BluePrints/OBJECTS/BP_button.parentPuzzle` self _asbp_button_3))

(event `self.Interact`
  (params (PlayerActor :type "Actor Object Reference") (InteractedButton :type "Actor Object Reference")))

(fn `OnRep_CurrentSequence`)

(fn `ResetPuzzle`
  (`parent.ResetPuzzle`)
  (`KismetArrayLibrary.Array_Clear` (`self.CurrentSequence`))
  (`KismetSystemLibrary.PrintString` "Почисщено"))

(fn `UserConstructionScript`
  (`parent.UserConstructionScript`))