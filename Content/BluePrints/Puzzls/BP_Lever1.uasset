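; BP_Lever1 is a lever puzzle Blueprint that checks whether the correct combination of levers is active.
; On Interaction from a BP_Lever, it recounts active correct and incorrect levers in LeverArray using each lever's IsCorrectLever and IsActivited flags.
; It calls SolvePuzzle when exactly one correct lever and no incorrect ones are active.
; Print strings provide debug output, including an error for non-lever callers.
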(event `self.ReceiveInteraction`
  (params (`Player Actor` :type "Actor Object Reference") (`Interacted Button` :type "Actor Object Reference"))
  (`KismetSystemLibrary.PrintString` "Hello")
  (cast `/Game/BluePrints/OBJECTS/BP_Lever` `Interacted Button`
    (:`then`
      (set `self.ActiveIncorrect` 0)
      (set `self.ActiveCorrect` 0)
      (for _array_element (`self.LeverArray`)
        (if (`/Game/BluePrints/OBJECTS/BP_Lever.isCorrectLever` _array_element)
          (if (`/Game/BluePrints/OBJECTS/BP_Lever.isActivited` _array_element)
            (bind _result (`/Engine/EditorBlueprintResources/StandardMacros.IncrementInt` (`self.ActiveCorrect`))
              (:`  `
                (`KismetSystemLibrary.PrintString` (`KismetStringLibrary.Conv_IntToString` _result)))))
          (elif (`/Game/BluePrints/OBJECTS/BP_Lever.isActivited` _array_element)
            (bind _result_2 (`/Engine/EditorBlueprintResources/StandardMacros.IncrementInt` (`self.ActiveIncorrect`))
              (:`  `
                (`KismetSystemLibrary.PrintString` (`KismetStringLibrary.Conv_IntToString` _result_2)))))))
      (if (and (== (`self.ActiveCorrect`) 1) (== (`self.ActiveIncorrect`) 0))
        (`self.SolvePuzzle`)))
    (:`CastFailed`
      (`KismetSystemLibrary.PrintString` "error"))))

(fn `UserConstructionScript`
  (`parent.UserConstructionScript`))