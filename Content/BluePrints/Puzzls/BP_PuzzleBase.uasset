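; Base puzzle actor with a replicated Inactive, Active, Solved or Failed state, leaving interaction and reset logic as empty events.
; Interact forwards through a server event to ReceiveInteraction; its Active-state check is disconnected.
; Solving notifies listeners and triggers linked actors, while failure resets to Active after a short delay.
; The state's OnRep recolors a status light and has a sound call on solve.
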(event `Server_OnInteract`
  (params (PlayerActor :type "Actor Object Reference") (InteractedActor :type "Actor Object Reference"))
  (`KismetSystemLibrary.PrintString` "Кнопка стукаж")
  (`self.ReceiveInteraction` PlayerActor InteractedActor))

(event `/Game/FirstPerson/Blueprints/BPI_Interact.Interact`
  (params (PlayerActor :type "Actor Object Reference") (InteractedButton :type "Actor Object Reference"))
  (`self.Server_OnInteract` PlayerActor InteractedButton))

(event `/Game/FirstPerson/Blueprints/BPI_PuzzleTriggerrable.TriggerActivation`
  (params (IsActivated :type Boolean)))

(event `ReceiveInteraction`
  (params (`Player Actor` :type "Actor Object Reference") (`Interacted Button` :type "Actor Object Reference")))

(event `OnResetLogic`)

(event `Server_HandleFailedState`
  (set `self.PuzzleState` "NewEnumerator3")
  (`KismetSystemLibrary.Delay` 2.0)
  (`self.ResetPuzzle`))

(fn `GetInteractText`
  (returns (Text :type Text))
  (return ""))

(fn `OnRep_PuzzleState`
  (bind _statuslight (`self.StatusLight`))
  (`KismetSystemLibrary.PrintString` "Hello")
  (switch `/Game/BluePrints/EnumS/E_PuzzleState` (`self.PuzzleState`)
    (:`NewEnumerator1`
      (`LightComponent.SetLightColor` _statuslight (struct :`G` 0.001623 :`B` 1.0 :`A` 1.0) true)
      (`KismetSystemLibrary.PrintString` "Kolir zmineno"))
    (:`NewEnumerator2`
      (`GameplayStatics.PlaySoundAtLocation` null (0.0 0.0 0.0) (struct) 1.0 1.0 0.0 null null null null)
      (`LightComponent.SetLightColor` _statuslight (struct :`R` 0.123424 :`G` 1.0 :`A` 1.0) true))
    (:`NewEnumerator3`
      (`LightComponent.SetLightColor` _statuslight (struct :`R` 0.21875 :`B` 0.01519 :`A` 1.0) true))))

(fn `ResetPuzzle`
  (set `self.PuzzleState` "NewEnumerator0")
  (set `self.PuzzleState` "NewEnumerator1"))

(fn `SolvePuzzle`
  (if (`|EnumInequality` (`self.PuzzleState`) "NewEnumerator2")
    (set `self.PuzzleState` "NewEnumerator2")
    (`self.OnPuzzleSolved` (`self.PuzzleID`))
    (for _array_element (`self.LinkedActors`)
      (message `/Game/FirstPerson/Blueprints/BPI_PuzzleTriggerrable.TriggerActivation` _array_element true))))

(fn `StartPuzzle`
  (switch `/Game/BluePrints/EnumS/E_PuzzleState` "NewEnumerator0"
    (:`NewEnumerator0`
      (set `self.PuzzleState` "NewEnumerator1")
      (`self.OnPuzzleStarted` (`self.PuzzleID`)))))

(fn `UserConstructionScript`)